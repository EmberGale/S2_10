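; AI pawn that wanders endlessly between random navmesh points within X/Y bounds, using its spawn height and FloatingPawnMovement.
; AI MoveTo picks a new point and repeats on success or failure.
; A capsule hit offsets the pawn by the normal impulse and changes the stored target without restarting the move.
; Tick turns it to face its velocity and shows debug text and shapes for target and heading.
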(event OnComponentHit(Capsule)
  (params (HitComponent :type Primitive%20Component%20Object%20Reference) (OtherActor :type Actor%20Object%20Reference) (OtherComp :type Primitive%20Component%20Object%20Reference) (NormalImpulse :type Vector :default "0, 0, 0") (Hit :type Hit%20Result%20Structure%20%28by%20ref%29))
  (Transformation|AddActorLocalOffset NormalImpulse true false)
  (Development|PrintText "Collision" true true "(R=0.000000,G=0.660000,B=1.000000,A=1.000000)" 0.5 "Collision")
  (bind _randompoint (CallFunction|GetRandomPoint))
  (Variables|Default|SetTargetPoint _randompoint)
  (Utilities|FlowControl|Delay 0.2))

(event Custom|MoveToTarget
  (AI|AIMoveTo self (Variables|Default|GetTargetPoint) 0 5.0 false
    (:OnSuccess
      _)
    (:OnFail
      _))
  (bind _randompoint (CallFunction|GetRandomPoint))
  (Variables|Default|SetTargetPoint _randompoint)
  (CallFunction|MovetoTarget))

(event EventBeginPlay
  (bind _randompoint (CallFunction|GetRandomPoint))
  (Variables|Default|SetTargetPoint _randompoint)
  (CallFunction|MovetoTarget))

(event EventTick
  (params (DeltaSeconds :type Float%20%28single-precision%29))
  (CallFunction|DebugLocation)
  (CallFunction|RotatetoVelocity))

(fn ConstructionScript
  (Variables|Default|SetZLevel (.z (.location (Transformation|GetActorTransform))))
  (Variables|/Script/Engine.FloatingPawnMovement|SetMaxSpeed (Variables|Default|GetFloatingPawnMovement) (Variables|Default|GetSpeed)))

(fn IsActorinBoundaries2D
  (params (Min%20X :type Float%20%28double-precision%29) (Max%20X :type Float%20%28double-precision%29) (Min%20Y :type Float%20%28double-precision%29) (Max%20Y :type Float%20%28double-precision%29))
  (bind _returnvalue (Transformation|GetActorLocation))
  (return (and (Math|Float|InRange(Float) (.x _returnvalue) Min%20X Max%20X) (Math|Float|InRange(Float) (.y _returnvalue) Min%20Y Max%20Y))))

(fn GetRandomPoint
  (return (.ProjectedLocation (AI|Navigation|ProjectPointtoNavigation (Math|Vector|MakeVector (Math|Random|RandomFloatinRange (Variables|Default|GetMin%20X) (Variables|Default|GetMax%20X)) (Math|Random|RandomFloatinRange (Variables|Default|GetMin%20Y) (Variables|Default|GetMax%20Y)) (Variables|Default|GetZLevel)) 0 0 "0, 0, 0"))))

(fn CheckBounds)

(fn DebugLocation
  (bind _returnvalue (Transformation|GetActorLocation))
  (bind _targetpoint (Variables|Default|GetTargetPoint))
  (Development|PrintText (Utilities|Text|FormatText "Target: {0}" (Utilities|Text|ToText(String) (Variables|Default|GetTargetPoint))) true true "(R=0.000000,G=0.660000,B=1.000000,A=1.000000)" 2.0 "Target")
  (Development|PrintText (Utilities|Text|FormatText "Actor location: {0}" (Utilities|Text|ToText(String) (Transformation|GetActorLocation))) true true "(R=0.000000,G=0.660000,B=1.000000,A=1.000000)" 2.0 "Actor location")
  (Development|PrintText (Utilities|Text|FormatText "Actor rotation: {0}" (.yaw (Transformation|GetActorRotation))) true true "(R=0.000000,G=0.660000,B=1.000000,A=1.000000)" 2.0 "Actor rotation")
  (Rendering|Debug|DrawDebugArrow _returnvalue (+ _returnvalue (* (Transformation|GetActorForwardVector) (LocalVariables|GetArrowLength))) 5e+01 "(R=0.243016,G=0.297848,B=1.000000,A=1.000000)" 0.0 1.0)
  (Class|VisualLoggerKismetLibrary|LogLocation 0 _targetpoint "" "(R=0.000000,G=0.000000,B=1.000000,A=1.000000)" 1e+01 "VisLogBP")
  (Rendering|Debug|DrawDebugSphere _targetpoint 3e+01 4 "(R=0.664557,G=1.000000,B=0.698986,A=1.000000)" 0.0))

(fn RotatetoVelocity
  (Transformation|SetActorRotation (Math|Rotator|FindLookatRotation (Math|Vector|VectorZero) (Transformation|GetVelocity))))