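; BP_Movable is an actor that wanders between random points inside an XY rectangle at the height captured in its construction script.
; Each Tick it faces the target and makes a swept step forward, snapping when close, and prints debug text.
; It picks a new point on BeginPlay, capsule hit, arrival or leaving bounds.
; The step divides Speed by DeltaSeconds, so shorter frames give larger steps.
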(event OnComponentHit(Capsule)
  (params (HitComponent :type Primitive%20Component%20Object%20Reference) (OtherActor :type Actor%20Object%20Reference) (OtherComp :type Primitive%20Component%20Object%20Reference) (NormalImpulse :type Vector :default "0, 0, 0") (Hit :type Hit%20Result%20Structure%20%28by%20ref%29))
  (Development|PrintText "Collision" true true "(R=0.000000,G=0.660000,B=1.000000,A=1.000000)" 0.5 "Collision")
  (bind _randompoint (CallFunction|GetRandomPoint))
  (Variables|Default|SetRandomPoint _randompoint))

(event EventBeginPlay
  (bind _randompoint (CallFunction|GetRandomPoint))
  (Variables|Default|SetRandomPoint _randompoint))

(event EventTick
  (params (DeltaSeconds :type Float%20%28single-precision%29))
  (CallFunction|CheckBoundsorReached)
  (CallFunction|Moveto (Variables|Default|GetRandomPoint) (/ (/ (Variables|Default|GetSpeed) 3.6e+03) DeltaSeconds))
  (CallFunction|DebugLocation))

(fn ConstructionScript
  (Variables|Default|SetZLevel (.z (.location (Transformation|GetActorTransform)))))

(fn IsActorinBoundaries2D
  (params (Min%20X :type Float%20%28double-precision%29) (Max%20X :type Float%20%28double-precision%29) (Min%20Y :type Float%20%28double-precision%29) (Max%20Y :type Float%20%28double-precision%29))
  (bind _returnvalue (Transformation|GetActorLocation))
  (return (and (Math|Float|InRange(Float) (.x _returnvalue) Min%20X Max%20X) (Math|Float|InRange(Float) (.y _returnvalue) Min%20Y Max%20Y))))

(fn GetRandomPoint
  (return (Math|Vector|MakeVector (Math|Random|RandomFloatinRange (Variables|Default|GetMin%20X) (Variables|Default|GetMax%20X)) (Math|Random|RandomFloatinRange (Variables|Default|GetMin%20Y) (Variables|Default|GetMax%20Y)) (Variables|Default|GetZLevel))))

(fn CheckBoundsorReached
  (if (and (CallFunction|IsActorinBoundaries2D (Variables|Default|GetMin%20X) (Variables|Default|GetMax%20X) (Variables|Default|GetMin%20Y) (Variables|Default|GetMax%20Y)) (not (Utilities|Operators|EqualEqual (Transformation|GetActorLocation) (Variables|Default|GetRandomPoint) 5.0)))
    _
    (else
      (bind _randompoint (CallFunction|GetRandomPoint))
      (Variables|Default|SetRandomPoint _randompoint)))
  (return))

(fn DebugLocation
  (Development|PrintText (Utilities|Text|FormatText "Target: {0}" (Utilities|Text|ToText(String) (Variables|Default|GetRandomPoint))) true true "(R=0.000000,G=0.660000,B=1.000000,A=1.000000)" 2.0 "Target")
  (Development|PrintText (Utilities|Text|FormatText "Actor location: {0}" (Utilities|Text|ToText(String) (Transformation|GetActorLocation))) true true "(R=0.000000,G=0.660000,B=1.000000,A=1.000000)" 2.0 "Actor location")
  (Development|PrintText (Utilities|Text|FormatText "Actor rotation: {0}" (.yaw (Transformation|GetActorRotation))) true true "(R=0.000000,G=0.660000,B=1.000000,A=1.000000)" 2.0 "Actor rotation"))

(fn Moveto
  (params (Target :type Vector) (Speed :type Float%20%28double-precision%29))
  (Utilities|FlowControl|Sequence
    (:then_0
      (Transformation|SetActorRotation (Math|Rotator|FindLookatRotation (Transformation|GetActorLocation) Target)))
    (:then_1
      ;[1 1 1] If distance > speed
      (if (> Speed (Math|Vector|Distance(Vector) Target (Transformation|GetActorLocation)))
        (Transformation|SetActorLocation Target true false)
        (else
          (Transformation|AddActorWorldOffset (* Speed (Transformation|GetActorForwardVector)) true))))))